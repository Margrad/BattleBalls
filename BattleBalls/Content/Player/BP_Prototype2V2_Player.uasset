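; Prototype player vehicle pawn, a physics-driven four-wheeled body with skid steering and a gimbal and spring-arm aim camera.
; Forward input pushes all wheels along the body's forward vector; right input drives left and right wheels oppositely.
; Forces taper toward speed and yaw-rate limits, while Tick multiplies body angular velocity by DeltaSeconds, heavily damping spin.
; GetBackUp zeroes yaw, keeping roll and pitch, then sets location using a raised Z.
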(event EventTick
  (params (DeltaSeconds :type Float%20%28single-precision%29))
  (Class|PrimitiveComponent|SetPhysicsAngularVelocityinDegrees (Variables|Default|GetBody) (* (Physics|GetPhysicsAngularVelocityinDegrees (Variables|Default|GetBody) "None") DeltaSeconds) false "None"))

(event Input|ActionEvents|InputActionGetBackUp
  (params (Key :type Key%20Structure))
  (bind _body (Variables|Default|GetBody))
  (bind _body_2 (Variables|Default|GetBody))
  (bind _returnvalue (Transformation|GetWorldRotation _body_2))
  (:Pressed
    (Utilities|FlowControl|Sequence
      (:then_0
        (Transformation|SetWorldRotation _body_2 (Math|Rotator|MakeRotator (.roll _returnvalue) (.pitch _returnvalue) 0.0) false false))
      (:then_1
        (Transformation|SetWorldLocation _body (Math|Vector|MakeVector 0.0 0.0 (+ (.z (Transformation|GetWorldLocation _body)) 1.0)) false false)))))

(event Input|AxisEvents|InputAxisAimAzimuth
  (params (AxisValue :type Float%20%28single-precision%29))
  ;[1 1 1] Camera Rotation
  (Transformation|AddLocalRotation (Variables|Default|GetGimbal) (Math|Rotator|MakeRotator 0.0 0.0 AxisValue) false false))

(event Input|AxisEvents|InputAxisMoveForward
  (params (AxisValue :type Float%20%28single-precision%29))
  ;[1 1 1] MovementInputs
  (CallFunction|IntendMoveForward AxisValue))

(event Input|AxisEvents|InputAxisMoveRight
  (params (AxisValue :type Float%20%28single-precision%29))
  ;[1 1 1] MovementInputs
  (CallFunction|IntendMoveRight AxisValue))

(event Input|AxisEvents|InputAxisAimElevation
  (params (AxisValue :type Float%20%28single-precision%29))
  ;[1 1 1] Camera Rotation
  (Transformation|AddLocalRotation (Variables|Default|GetSpringArm) (Math|Rotator|MakeRotator 0.0 AxisValue 0.0) false false))

(fn ConstructionScript)

(fn IntendMoveForward
  (params (Throttle :type Float%20%28single-precision%29))
  (bind _returnvalue (Transformation|GetVelocity))
  (bind _basethrottle (Variables|Default|GetBaseThrottle))
  (bind _maxspeed (Variables|Default|GetMaxSpeed))
  (bind _returnvalue_2 (Math|Vector|VectorLength _returnvalue))
  (bind _returnvalue_3 (/ _returnvalue_2 _maxspeed))
  (bind _returnvalue_4 (- 1.0 _returnvalue_3))
  (bind _returnvalue_5 (Math|Float|Clamp(Float) _returnvalue_4))
  (bind _returnvalue_6 (* _returnvalue_5 _basethrottle))
  (bind _returnvalue_7 (* Throttle _returnvalue_6))
  (Utilities|FlowControl|Sequence
    (:then_0
      (Physics|AddForce (Variables|Default|GetLFWheel) (* (Math|Vector|GetForwardVector (Variables|Default|GetBody)) _returnvalue_7) "None" false))
    (:then_1
      (Physics|AddForce (Variables|Default|GetLBWheel) (* (Math|Vector|GetForwardVector (Variables|Default|GetBody)) _returnvalue_7) "None" false))
    (:then_2
      (Physics|AddForce (Variables|Default|GetRFWheel) (* (Math|Vector|GetForwardVector (Variables|Default|GetBody)) _returnvalue_7) "None" false))
    (:then_3
      (Physics|AddForce (Variables|Default|GetRBWheel) (* (Math|Vector|GetForwardVector (Variables|Default|GetBody)) _returnvalue_7) "None" false))))

(fn IntendMoveRight
  (params (Throttle :type Float%20%28single-precision%29))
  (bind _basethrottle (Variables|Default|GetBaseThrottle))
  (bind _maxrotation (Variables|Default|GetMaxRotation))
  (bind _body (Variables|Default|GetBody))
  (bind _returnvalue (Physics|GetPhysicsAngularVelocityinDegrees _body "None"))
  (bind _returnvalue_2 (Math|Float|Absolute(Float) (.z _returnvalue)))
  (bind _returnvalue_3 (/ _returnvalue_2 _maxrotation))
  (bind _returnvalue_4 (- 1.0 _returnvalue_3))
  (bind _returnvalue_5 (Math|Float|Clamp(Float) _returnvalue_4))
  (bind _returnvalue_6 (* _returnvalue_5 _basethrottle))
  (bind _returnvalue_7 (* Throttle _returnvalue_6))
  (bind _returnvalue_8 (* _returnvalue_7 -1.0))
  (Utilities|FlowControl|Sequence
    (:then_0
      (Physics|AddForce (Variables|Default|GetLFWheel) (* (Math|Vector|GetForwardVector (Variables|Default|GetBody)) _returnvalue_7) "None" false))
    (:then_1
      (Physics|AddForce (Variables|Default|GetLBWheel) (* (Math|Vector|GetForwardVector (Variables|Default|GetBody)) _returnvalue_7) "None" false))
    (:then_2
      (Physics|AddForce (Variables|Default|GetRFWheel) (* (Math|Vector|GetForwardVector (Variables|Default|GetBody)) _returnvalue_8) "None" false))
    (:then_3
      (Physics|AddForce (Variables|Default|GetRBWheel) (* (Math|Vector|GetForwardVector (Variables|Default|GetBody)) _returnvalue_8) "None" false))))