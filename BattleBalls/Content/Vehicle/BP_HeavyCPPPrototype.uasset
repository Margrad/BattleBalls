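; Heavy vehicle pawn prototype, apparently on a C++ base, that maps player input to driving, camera aim and weapon fire.
; Move axes send forward and turn intent to MovementComponent, and the GetBackUp action calls its side-righting function.
; Aim azimuth yaws the Gizmoball and elevation pitches the SpringArm, keeping the two rotation axes on separate components.
; Fire triggers WeaponComponent, while EventGraph and construction script are empty.
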(event EventBeginPlay)

(event Collision|EventActorBeginOverlap
  (params (OtherActor :type Actor%20Object%20Reference)))

(event EventTick
  (params (DeltaSeconds :type Float%20%28single-precision%29)))

(event Input|ActionEvents|InputActionGetBackUp
  (params (Key :type Key%20Structure))
  ;[1 1 1] Action keys
  (:Pressed
    (Class|VehicleNavMovementComponent|GetBackUpSide (Variables|Default|GetMovementComponent))))

(event Input|ActionEvents|InputActionFire
  (params (Key :type Key%20Structure))
  ;[1 1 1] Action keys
  (:Pressed
    (Class|WeaponComponent|Fire (Variables|Default|GetWeaponComponent))))

(event Input|AxisEvents|InputAxisMoveForward
  (params (AxisValue :type Float%20%28single-precision%29))
  ;[1 1 1] Movement inputs
  (Class|VehicleNavMovementComponent|IntendMoveForward (Variables|Default|GetMovementComponent) AxisValue))

(event Input|AxisEvents|InputAxisMoveRight
  (params (AxisValue :type Float%20%28single-precision%29))
  ;[1 1 1] Movement inputs
  (Class|VehicleNavMovementComponent|IntendTurnRight (Variables|Default|GetMovementComponent) AxisValue))

(event Input|AxisEvents|InputAxisAimAzimuth
  (params (AxisValue :type Float%20%28single-precision%29))
  ;[1 1 1] Camera Movement
  (Transformation|AddLocalRotation (Variables|Default|GetGizmoball) (Math|Rotator|MakeRotator 0.0 0.0 AxisValue) false false))

(event Input|AxisEvents|InputAxisAimElevation
  (params (AxisValue :type Float%20%28single-precision%29))
  ;[1 1 1] Camera Movement
  (Transformation|AddLocalRotation (Variables|Default|GetSpringArm) (Math|Rotator|MakeRotator 0.0 AxisValue 0.0) false false))

(fn ConstructionScript)