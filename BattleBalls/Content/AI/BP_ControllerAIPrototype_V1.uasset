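; Prototype AI controller for BP_Prototype2V2_AI pawns that drives their decisions and rights them when they flip over.
; On BeginPlay it loads BaseBlackboard and runs the BallsDecisionTree behavior tree.
; Each Tick it calls PopBackUp on the pawn when IsUpSideDown reports a flip.
; That check relies on roll in practice, since its pitch threshold lies beyond any reachable angle.
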(event EventTick
  (params (DeltaSeconds :type Float%20%28single-precision%29))
  (bind (_returnvalue _returnvalue2) (CallFunction|IsUpSideDown))
  (bind _asbp_prototype_2v2_ai (Utilities|Casting|CastToBP_Prototype2V2_AI _returnvalue))
  (if _returnvalue2
    (Default|PopBackUp _asbp_prototype_2v2_ai)))

(event EventBeginPlay
  (Class|AIController|UseBlackboard "/Game/AI/AIDecisionMAking/BaseBlackboard.BaseBlackboard")
  (AI|RunBehaviorTree "/Game/AI/AIDecisionMAking/BallsDecisionTree.BallsDecisionTree"))

(fn ConstructionScript)

(fn IsUpSideDown
  (bind _returnvalue (Pawn|GetControlledPawn))
  (bind _returnvalue_2 (Transformation|GetActorRotation _returnvalue))
  (return _returnvalue (or (>= (Math|Float|Absolute(Float) (.roll _returnvalue_2)) 1.2e+02) (>= (Math|Float|Absolute(Float) (.pitch _returnvalue_2)) 1.2e+03))))