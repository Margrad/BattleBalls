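; BP_Prototype is a player-controlled wheeled vehicle pawn with a switchable first- and third-person camera.
; On BeginPlay it passes its left and right wheels to SetWheels, and movement axes forward to intend-move functions whose logic lives outside these graphs.
; Aim axes yaw the Gimbal and pitch the SpringArm separately, while CameraChange toggles the view by changing the spring arm length.
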(event EventBeginPlay
  (Class|VehicleBase|SetWheels (Variables|Default|GetLeftWheels) (Variables|Default|GetRightWheels)))

(event Input|ActionEvents|InputActionCameraChange
  (params (Key :type Key%20Structure))
  ;[1 1 1] Set Camera between 1st and 3rd Person
  (:Pressed
    (if (Variables|Default|GetIsFPCamera)
      (Variables|/Script/Engine.SpringArmComponent|SetTargetArmLength (Variables|Default|GetSpringArm) 3e+02)
      (Variables|Default|SetIsFPCamera false)
      (else
        (Variables|/Script/Engine.SpringArmComponent|SetTargetArmLength (Variables|Default|GetSpringArm) -1e+01)
        (Variables|Default|SetIsFPCamera true)))))

(event Input|AxisEvents|InputAxisAimAzimuth
  (params (AxisValue :type Float%20%28single-precision%29))
  ;[1 1 1] Camera Rotation
  (Transformation|AddLocalRotation (Variables|Default|GetGimbal) (Math|Rotator|MakeRotator 0.0 0.0 AxisValue) false false))

(event Input|AxisEvents|InputAxisAimElevation
  (params (AxisValue :type Float%20%28single-precision%29))
  ;[1 1 1] Camera Rotation
  (Transformation|AddLocalRotation (Variables|Default|GetSpringArm) (Math|Rotator|MakeRotator 0.0 AxisValue 0.0) false false))

(event Input|AxisEvents|InputAxisMoveForward
  (params (AxisValue :type Float%20%28single-precision%29))
  (Class|VehicleBase|IntendMoveForward AxisValue))

(event Input|AxisEvents|InputAxisMoveRight
  (params (AxisValue :type Float%20%28single-precision%29))
  (Class|VehicleBase|IndendMoveRigth AxisValue))

(fn ConstructionScript)