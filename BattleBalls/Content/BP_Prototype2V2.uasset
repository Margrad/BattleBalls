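; Prototype player-driven four-wheeled physics vehicle with skid steering and an orbit camera on a gimbal and spring arm.
; Move inputs push each wheel along the body's forward axis, with left and right sides opposed for turning.
; Throttle fades linearly as speed or yaw rate nears its maximum.
; Tick rewrites the body's angular velocity using a tenth of its current Y (pitch) rate.
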(event EventTick
  (params (DeltaSeconds :type Float%20%28single-precision%29))
  (Class|PrimitiveComponent|SetPhysicsAngularVelocityinDegrees (Variables|Default|GetBody) (Math|Vector|MakeVector 0.0 (* (.y (Physics|GetPhysicsAngularVelocityinDegrees (Variables|Default|GetBody) "None")) 0.1) 0.0) false "None"))

(event Input|AxisEvents|InputAxisAimAzimuth
  (params (AxisValue :type Float%20%28single-precision%29))
  ;[1 1 1] Camera Rotation
  (Transformation|AddLocalRotation (Variables|Default|GetGimbal) (Math|Rotator|MakeRotator 0.0 0.0 AxisValue) false false))

(event Input|AxisEvents|InputAxisMoveForward
  (params (AxisValue :type Float%20%28single-precision%29))
  (CallFunction|IntendMoveForward (* AxisValue (* (Math|Float|Clamp(Float) (- 1.0 (/ (Math|Vector|VectorLength (Transformation|GetVelocity)) (Variables|Default|GetMaxSpeed)))) (Variables|Default|GetBaseThrottle)))))

(event Input|AxisEvents|InputAxisMoveRight
  (params (AxisValue :type Float%20%28single-precision%29))
  (CallFunction|IntendMoveRight (* AxisValue (* (Math|Float|Clamp(Float) (- 1.0 (/ (Math|Float|Absolute(Float) (.z (Physics|GetPhysicsAngularVelocityinDegrees (Variables|Default|GetBody) "None"))) (Variables|Default|GetMaxRotation)))) (Variables|Default|GetBaseThrottle)))))

(event Input|AxisEvents|InputAxisAimElevation
  (params (AxisValue :type Float%20%28single-precision%29))
  ;[1 1 1] Camera Rotation
  (Transformation|AddLocalRotation (Variables|Default|GetSpringArm) (Math|Rotator|MakeRotator 0.0 AxisValue 0.0) false false))

(fn ConstructionScript)

(fn IntendMoveForward
  (params (Throttle :type Float%20%28single-precision%29))
  (Utilities|FlowControl|Sequence
    (:then_0
      (Physics|AddForce (Variables|Default|GetLFWheel) (* (Math|Vector|GetForwardVector (Variables|Default|GetBody)) Throttle) "None" false))
    (:then_1
      (Physics|AddForce (Variables|Default|GetLBWheel) (* (Math|Vector|GetForwardVector (Variables|Default|GetBody)) Throttle) "None" false))
    (:then_2
      (Physics|AddForce (Variables|Default|GetRFWheel) (* (Math|Vector|GetForwardVector (Variables|Default|GetBody)) Throttle) "None" false))
    (:then_3
      (Physics|AddForce (Variables|Default|GetRBWheel) (* (Math|Vector|GetForwardVector (Variables|Default|GetBody)) Throttle) "None" false))))

(fn IntendMoveRight
  (params (Throttle :type Float%20%28single-precision%29))
  (bind _returnvalue (* Throttle -1.0))
  (Utilities|FlowControl|Sequence
    (:then_0
      (Physics|AddForce (Variables|Default|GetLFWheel) (* (Math|Vector|GetForwardVector (Variables|Default|GetBody)) Throttle) "None" false))
    (:then_1
      (Physics|AddForce (Variables|Default|GetLBWheel) (* (Math|Vector|GetForwardVector (Variables|Default|GetBody)) Throttle) "None" false))
    (:then_2
      (Physics|AddForce (Variables|Default|GetRFWheel) (* (Math|Vector|GetForwardVector (Variables|Default|GetBody)) _returnvalue) "None" false))
    (:then_3
      (Physics|AddForce (Variables|Default|GetRBWheel) (* (Math|Vector|GetForwardVector (Variables|Default|GetBody)) _returnvalue) "None" false))))